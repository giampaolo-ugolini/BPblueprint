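; BP_Fragment_09 is a clickable mirror fragment in the mirror repair game that starts with the Gradient_Star material.
; A click is ignored if its material is RepairedFragment, another selection is flagged in BP_MirrorGame, or all fragments are repaired.
; Otherwise it parses its ID from its display name into BP_MirrorGame and flags the selection.
; It also moves the shared BP_FragmentLight spotlight above itself and brightens it.
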(event `self.ReceiveBeginPlay`
  (`PrimitiveComponent.SetMaterial` (`self.Fragment_09`) 0 "/Engine/MaterialTemplates/Gradients/Gradient_Star.Gradient_Star"))

(event `self.ReceiveActorOnClicked`
  (params (ButtonPressed :type "Key Structure"))
  (if (`KismetStringLibrary.NotEqual_StrStr` (`KismetSystemLibrary.GetDisplayName` (`PrimitiveComponent.GetMaterial` (`self.Fragment_09`) 0)) "RepairedFragment")
    (bind _returnvalue (`GameplayStatics.GetActorOfClass` "/Game/Blueprints/BP_MirrorGame.BP_MirrorGame_C"))
    (if (== (`/Game/Blueprints/BP_MirrorGame.StatusOfFragment` _returnvalue) 0)
      (bind _returnvalue_2 (`GameplayStatics.GetActorOfClass` "/Game/Blueprints/BP_MirrorGame.BP_MirrorGame_C"))
      (if (< (`/Game/Blueprints/BP_MirrorGame.RepairStatus` _returnvalue_2) (`/Game/Blueprints/BP_MirrorGame.TotalFragments` _returnvalue_2))
        (bind _returnvalue_3 (`GameplayStatics.GetActorOfClass` "/Game/Blueprints/BP_MirrorGame.BP_MirrorGame_C"))
        (bind _output_get (set `/Game/Blueprints/BP_MirrorGame.FragmentID` (`KismetStringLibrary.Conv_StringToInt` (`KismetStringLibrary.GetSubstring` (`KismetSystemLibrary.GetDisplayName` self) 12 2)) _returnvalue_3))
        (`KismetSystemLibrary.PrintString` (`KismetStringLibrary.Conv_IntToString` _output_get))
        (bind _returnvalue_4 (`GameplayStatics.GetActorOfClass` "/Game/Blueprints/MirrorBluePrints/BP_FragmentLight.BP_FragmentLight_C"))
        (`self.K2_SetActorLocation` _returnvalue_4 (+ (`self.K2_GetActorLocation` self) (0.0 0.0 500.0)) false false)
        (`LightComponent.SetIntensity` (`/Game/Blueprints/MirrorBluePrints/BP_FragmentLight.SpotLight` _returnvalue_4) 1000000.0)
        (bind _returnvalue_5 (`GameplayStatics.GetActorOfClass` "/Game/Blueprints/BP_MirrorGame.BP_MirrorGame_C"))
        (set `/Game/Blueprints/BP_MirrorGame.StatusOfFragment` 1 _returnvalue_5)))))

(fn `UserConstructionScript`)