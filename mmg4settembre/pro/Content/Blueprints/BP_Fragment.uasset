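; BP_Fragment is a mirror fragment actor, apparently for a mirror repair puzzle, that currently only prints its display name when clicked.
; All other logic is disconnected and never runs.
; Those leftover drafts track the active fragment, status and ID through BP_MirrorGame, found with GetActorOfClass and matched by display-name strings.
; They move the fragment with MoveComponentTo to lift it or fit it into the mirror.
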(event `self.ReceiveBeginPlay`)

(event `self.ReceiveActorOnClicked`
  (params (ButtonPressed :type "Key Structure"))
  (`KismetSystemLibrary.PrintString` (`KismetSystemLibrary.GetDisplayName` self)))

(fn `UserConstructionScript`)