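; BP_MirrorGame_MG manages a mirror-repair minigame, tracking fragment progress and the active fragment and target names.
; FinalRepairPhase checks RepairStatus against TotalFragments, then after a short delay hides twenty fragment actors, each found by its own class.
; WorkedFragmentUpdate builds zero-padded fragment and target names from FragmentID.
; Update is a rougher variant that resets FragmentID and prints the fragment name.
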(event `FinalRepairPhase`
  (if (== (`self.RepairStatus`) (`self.TotalFragments`))
    (`KismetSystemLibrary.Delay` 1.5)
    (bind _returnvalue (`GameplayStatics.GetActorOfClass` "/Game/Blueprints/MirrorBluePrints/BP_Fragment_00_MG.BP_Fragment_00_MG_C"))
    (`self.SetActorHiddenInGame` _returnvalue true)
    (bind _returnvalue_2 (`GameplayStatics.GetActorOfClass` "/Game/Blueprints/MirrorBluePrints/BP_Fragment_01_MG.BP_Fragment_01_MG_C"))
    (`self.SetActorHiddenInGame` _returnvalue_2 true)
    (bind _returnvalue_3 (`GameplayStatics.GetActorOfClass` "/Game/Blueprints/MirrorBluePrints/BP_Fragment_02_MG.BP_Fragment_02_MG_C"))
    (`self.SetActorHiddenInGame` _returnvalue_3 true)
    (bind _returnvalue_4 (`GameplayStatics.GetActorOfClass` "/Game/Blueprints/MirrorBluePrints/BP_Fragment_03_MG.BP_Fragment_03_MG_C"))
    (`self.SetActorHiddenInGame` _returnvalue_4 true)
    (bind _returnvalue_5 (`GameplayStatics.GetActorOfClass` "/Game/Blueprints/MirrorBluePrints/BP_Fragment_04_MG.BP_Fragment_04_MG_C"))
    (`self.SetActorHiddenInGame` _returnvalue_5 true)
    (bind _returnvalue_6 (`GameplayStatics.GetActorOfClass` "/Game/Blueprints/MirrorBluePrints/BP_Fragment_05_MG.BP_Fragment_05_MG_C"))
    (`self.SetActorHiddenInGame` _returnvalue_6 true)
    (bind _returnvalue_7 (`GameplayStatics.GetActorOfClass` "/Game/Blueprints/MirrorBluePrints/BP_Fragment_06_MG.BP_Fragment_06_MG_C"))
    (`self.SetActorHiddenInGame` _returnvalue_7 true)
    (bind _returnvalue_8 (`GameplayStatics.GetActorOfClass` "/Game/Blueprints/MirrorBluePrints/BP_Fragment_07_MG.BP_Fragment_07_MG_C"))
    (`self.SetActorHiddenInGame` _returnvalue_8 true)
    (bind _returnvalue_9 (`GameplayStatics.GetActorOfClass` "/Game/Blueprints/MirrorBluePrints/BP_Fragment_08_MG.BP_Fragment_08_MG_C"))
    (`self.SetActorHiddenInGame` _returnvalue_9 true)
    (bind _returnvalue_10 (`GameplayStatics.GetActorOfClass` "/Game/Blueprints/MirrorBluePrints/BP_Fragment_09_MG.BP_Fragment_09_MG_C"))
    (`self.SetActorHiddenInGame` _returnvalue_10 true)
    (bind _returnvalue_11 (`GameplayStatics.GetActorOfClass` "/Game/Blueprints/MirrorBluePrints/BP_Fragment_10_MG.BP_Fragment_10_MG_C"))
    (`self.SetActorHiddenInGame` _returnvalue_11 true)
    (bind _returnvalue_12 (`GameplayStatics.GetActorOfClass` "/Game/Blueprints/MirrorBluePrints/BP_Fragment_11_MG.BP_Fragment_11_MG_C"))
    (`self.SetActorHiddenInGame` _returnvalue_12 true)
    (bind _returnvalue_13 (`GameplayStatics.GetActorOfClass` "/Game/Blueprints/MirrorBluePrints/BP_Fragment_12_MG.BP_Fragment_12_MG_C"))
    (`self.SetActorHiddenInGame` _returnvalue_13 true)
    (bind _returnvalue_14 (`GameplayStatics.GetActorOfClass` "/Game/Blueprints/MirrorBluePrints/BP_Fragment_13_MG.BP_Fragment_13_MG_C"))
    (`self.SetActorHiddenInGame` _returnvalue_14 true)
    (bind _returnvalue_15 (`GameplayStatics.GetActorOfClass` "/Game/Blueprints/MirrorBluePrints/BP_Fragment_14_MG.BP_Fragment_14_MG_C"))
    (`self.SetActorHiddenInGame` _returnvalue_15 true)
    (bind _returnvalue_16 (`GameplayStatics.GetActorOfClass` "/Game/Blueprints/MirrorBluePrints/BP_Fragment_15_MG.BP_Fragment_15_MG_C"))
    (`self.SetActorHiddenInGame` _returnvalue_16 true)
    (bind _returnvalue_17 (`GameplayStatics.GetActorOfClass` "/Game/Blueprints/MirrorBluePrints/BP_Fragment_16_MG.BP_Fragment_16_MG_C"))
    (`self.SetActorHiddenInGame` _returnvalue_17 true)
    (bind _returnvalue_18 (`GameplayStatics.GetActorOfClass` "/Game/Blueprints/MirrorBluePrints/BP_Fragment_17_MG.BP_Fragment_17_MG_C"))
    (`self.SetActorHiddenInGame` _returnvalue_18 true)
    (bind _returnvalue_19 (`GameplayStatics.GetActorOfClass` "/Game/Blueprints/MirrorBluePrints/BP_Fragment_18_MG.BP_Fragment_18_MG_C"))
    (`self.SetActorHiddenInGame` _returnvalue_19 true)
    (bind _returnvalue_20 (`GameplayStatics.GetActorOfClass` "/Game/Blueprints/MirrorBluePrints/BP_Fragment_19_MG.BP_Fragment_19_MG_C"))
    (`self.SetActorHiddenInGame` _returnvalue_20 true)))

(fn `Update`
  (bind _result (`/Engine/EditorBlueprintResources/StandardMacros.IncrementInt` (`self.FragmentID`))
    (:`  `
      (if (< _result (`self.TotalFragments`))
        (set `self.ActiveFragment` "BP_Fragment_")
        (bind _output_get (set `self.FragmentID` 0))
        (bind _result_2 (`/Engine/EditorBlueprintResources/StandardMacros.IncrementInt` _output_get)
          (:`  `
            (if (< _result_2 10)
              (set `self.ActiveFragment` (`KismetStringLibrary.Concat_StrStr` (`self.ActiveFragment`) "0"))
              (bind _output_get_2 (set `self.ActiveFragment` (`KismetStringLibrary.Concat_StrStr` (`self.ActiveFragment`) (`KismetStringLibrary.Conv_IntToString` (`self.FragmentID`)))))
              (`KismetSystemLibrary.PrintString` _output_get_2))))))))

(fn `UserConstructionScript`)

(fn `WorkedFragmentUpdate`
  (bind _fragmentid (`self.FragmentID`))
  (if (< _fragmentid 10)
    (set `self.ActiveFragment` (`KismetStringLibrary.Concat_StrStr` "BP_Fragment_" "0" (`KismetStringLibrary.Conv_IntToString` _fragmentid)))
    (set `self.ActiveTarget` (`KismetStringLibrary.Concat_StrStr` "BP_Target_" "0" (`KismetStringLibrary.Conv_IntToString` _fragmentid)))
    (else
      (set `self.ActiveFragment` (`KismetStringLibrary.Concat_StrStr` "BP_Fragment_" (`KismetStringLibrary.Conv_IntToString` _fragmentid)))
      (set `self.ActiveTarget` (`KismetStringLibrary.Concat_StrStr` "BP_Target_" (`KismetStringLibrary.Conv_IntToString` _fragmentid))))))