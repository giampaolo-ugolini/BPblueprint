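; Clickable target slot in the mirror repair minigame that accepts fragment 00 when it is the expected piece.
; On click, it compares a number parsed from its display name with the FragmentID on BP_MirrorGame_MG.
; A match moves the fragment into place, applies the repaired material, turns off the fragment light, advances the game state and calls FinalRepairPhase.
; A mismatch temporarily swaps the target's material for three seconds.
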(event `self.ReceiveActorOnClicked`
  (params (ButtonPressed :type "Key Structure"))
  (bind _returnvalue (`GameplayStatics.GetActorOfClass` "/Game/Blueprints/BP_MirrorGame_MG.BP_MirrorGame_MG_C"))
  (if (== (`/Game/Blueprints/BP_MirrorGame_MG.FragmentID` _returnvalue) (`KismetStringLibrary.Conv_StringToInt` (`KismetStringLibrary.GetSubstring` (`KismetSystemLibrary.GetDisplayName` self) 10 2)))
    (bind _returnvalue_2 (`GameplayStatics.GetActorOfClass` "/Game/Blueprints/MirrorBluePrints/BP_Fragment_00_MG.BP_Fragment_00_MG_C"))
    (bind _fragment_00 (`/Game/Blueprints/MirrorBluePrints/BP_Fragment_00_MG.Fragment_00` _returnvalue_2))
    (`KismetSystemLibrary.MoveComponentTo` _fragment_00 (4000.0 0.0 -1000.0) (struct :`Pitch` 360.0 :`Yaw` 180.0 :`Roll` -270.0) false false 1.0)
    (`KismetSystemLibrary.Delay` 1.0)
    (bind _returnvalue_3 (`KismetMathLibrary.MakeVector` (.z (- (`self.K2_GetActorLocation`) (`self.K2_GetActorLocation` _returnvalue_2))) (.x (- (`self.K2_GetActorLocation`) (`self.K2_GetActorLocation` _returnvalue_2))) (.y (- (`self.K2_GetActorLocation`) (`self.K2_GetActorLocation` _returnvalue_2)))))
    (`KismetSystemLibrary.MoveComponentTo` _fragment_00 _returnvalue_3 (struct :`Pitch` 360.0 :`Yaw` 180.0 :`Roll` -270.0))
    (`GameplayStatics.PlaySound2D` "/Engine/VREditor/Sounds/VR_open.VR_open" 1.0 1.0 0.0 null null)
    (`self.K2_AddActorLocalOffset` (- _returnvalue_3 (0.0 50.0 0.0)))
    (`PrimitiveComponent.SetMaterial` _fragment_00 0 "/Game/Materials/RepairedFragment.RepairedFragment")
    (bind _returnvalue_4 (`GameplayStatics.GetActorOfClass` "/Game/Blueprints/MirrorBluePrints/BP_FragmentLight_MG.BP_FragmentLight_MG_C"))
    (`LightComponent.SetIntensity` (`/Game/Blueprints/MirrorBluePrints/BP_FragmentLight_MG.SpotLight` _returnvalue_4) 0.0)
    (bind _returnvalue_5 (`GameplayStatics.GetActorOfClass` "/Game/Blueprints/BP_MirrorGame_MG.BP_MirrorGame_MG_C"))
    (set `/Game/Blueprints/BP_MirrorGame_MG.StatusOfFragment` 0 _returnvalue_5)
    (bind _result (`/Engine/EditorBlueprintResources/StandardMacros.IncrementInt` (`/Game/Blueprints/BP_MirrorGame_MG.RepairStatus` _returnvalue_5))
      (:`  `
        (set `/Game/Blueprints/BP_MirrorGame_MG.RepairStatus` _result _returnvalue_5)
        (bind _result_2 (`/Engine/EditorBlueprintResources/StandardMacros.IncrementInt` (`/Game/Blueprints/BP_MirrorGame_MG.FragmentID` _returnvalue_5))
          (:`  `
            (set `/Game/Blueprints/BP_MirrorGame_MG.FragmentID` _result_2 _returnvalue_5)
            (bind _returnvalue_6 (`GameplayStatics.GetActorOfClass` "/Game/Blueprints/BP_MirrorGame_MG.BP_MirrorGame_MG_C"))
            (`/Game/Blueprints/BP_MirrorGame_MG.FinalRepairPhase` _returnvalue_6)))))
    (else
      (`PrimitiveComponent.SetMaterial` (`self.Target_00`) 0 "/Engine/VREditor/LaserPointer/LaserPointerMaterialInst.LaserPointerMaterialInst")
      (`KismetSystemLibrary.Delay` 3.0)
      (`PrimitiveComponent.SetMaterial` (`self.Target_00`) 0 "/Engine/Engine_MI_Shaders/M_Shader_SimpleTranslucent.M_Shader_SimpleTranslucent"))))

(fn `UserConstructionScript`)