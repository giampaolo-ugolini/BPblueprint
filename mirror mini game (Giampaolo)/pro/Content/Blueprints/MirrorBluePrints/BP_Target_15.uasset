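; Clickable target slot 15 in the mirror repair puzzle, which accepts its fragment only when BP_MirrorGame's current FragmentID matches.
; The expected ID is parsed from the actor's own display name.
; On a match it animates Fragment15 toward the target, offsets itself, applies the repaired material, turns off the fragment spotlight and updates the game's status and counters.
; Otherwise the target shows the laser pointer material briefly, then reverts.
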(event `self.ReceiveBeginPlay`
  (`PrimitiveComponent.SetMaterial` (`self.Target_15`) 0 "/Game/Materials/FragmentSelected.FragmentSelected"))

(event `self.ReceiveActorOnClicked`
  (params (ButtonPressed :type "Key Structure"))
  (bind _returnvalue (`GameplayStatics.GetActorOfClass` "/Game/Blueprints/BP_MirrorGame.BP_MirrorGame_C"))
  (if (== (`/Game/Blueprints/BP_MirrorGame.FragmentID` _returnvalue) (`KismetStringLibrary.Conv_StringToInt` (`KismetStringLibrary.GetSubstring` (`KismetSystemLibrary.GetDisplayName` self) 10 2)))
    (bind _returnvalue_2 (`GameplayStatics.GetActorOfClass` "/Game/Blueprints/MirrorBluePrints/BP_Fragment_15.BP_Fragment_15_C"))
    (bind _fragment_15 (`/Game/Blueprints/MirrorBluePrints/BP_Fragment_15.Fragment_15` _returnvalue_2))
    (`KismetSystemLibrary.MoveComponentTo` _fragment_15 (4000.0 0.0 0.0) (struct :`Pitch` 360.0 :`Yaw` 180.0 :`Roll` -270.0) false false 1.0)
    (`KismetSystemLibrary.Delay` 1.0)
    (bind _returnvalue_3 (`KismetMathLibrary.MakeVector` (.z (- (`self.K2_GetActorLocation`) (`self.K2_GetActorLocation` _returnvalue_2))) (.x (- (`self.K2_GetActorLocation`) (`self.K2_GetActorLocation` _returnvalue_2))) (.y (- (`self.K2_GetActorLocation`) (`self.K2_GetActorLocation` _returnvalue_2)))))
    (`KismetSystemLibrary.MoveComponentTo` _fragment_15 _returnvalue_3 (struct :`Pitch` 360.0 :`Yaw` 180.0 :`Roll` -270.0))
    (`self.K2_AddActorLocalOffset` (- _returnvalue_3 (0.0 50.0 0.0)))
    (`PrimitiveComponent.SetMaterial` _fragment_15 0 "/Game/Materials/RepairedFragment.RepairedFragment")
    (bind _returnvalue_4 (`GameplayStatics.GetActorOfClass` "/Game/Blueprints/MirrorBluePrints/BP_FragmentLight.BP_FragmentLight_C"))
    (`LightComponent.SetIntensity` (`/Game/Blueprints/MirrorBluePrints/BP_FragmentLight.SpotLight` _returnvalue_4) 0.0)
    (bind _returnvalue_5 (`GameplayStatics.GetActorOfClass` "/Game/Blueprints/BP_MirrorGame.BP_MirrorGame_C"))
    (set `/Game/Blueprints/BP_MirrorGame.StatusOfFragment` 0 _returnvalue_5)
    (bind _result (`/Engine/EditorBlueprintResources/StandardMacros.IncrementInt` (`/Game/Blueprints/BP_MirrorGame.RepairStatus` _returnvalue_5))
      (:`  `
        (set `/Game/Blueprints/BP_MirrorGame.RepairStatus` _result _returnvalue_5)
        (bind _result_2 (`/Engine/EditorBlueprintResources/StandardMacros.IncrementInt` (`/Game/Blueprints/BP_MirrorGame.FragmentID` _returnvalue_5))
          (:`  `
            (set `/Game/Blueprints/BP_MirrorGame.FragmentID` _result_2 _returnvalue_5)))))
    (else
      (`PrimitiveComponent.SetMaterial` (`self.Target_15`) 0 "/Engine/VREditor/LaserPointer/LaserPointerMaterialInst.LaserPointerMaterialInst")
      (`KismetSystemLibrary.Delay` 3.0)
      (`PrimitiveComponent.SetMaterial` (`self.Target_15`) 0 "/Game/Materials/FragmentSelected.FragmentSelected"))))

(fn `UserConstructionScript`)