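; BP_MirrorGame is a work-in-progress controller for what appears to be a mirror-fragment puzzle.
; BeginPlay applies a cloth material to its mesh, resets FragmentID and calls WorkedFragmentUpdate, which builds zero-padded active fragment and target names from the ID.
; Disconnected EventGraph logic matches fragments by display name, repositions them and animates the active one to its start location.
; A separate Update function, uncalled here, holds another version of the name-building logic.
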(event `self.ReceiveBeginPlay`
  (`PrimitiveComponent.SetMaterial` (`self.StaticMeshComponent`) 0 "/Game/Materials/M_Cloth.M_Cloth")
  (set `self.FragmentID` 0)
  (`self.WorkedFragmentUpdate`))

(fn `Update`
  (bind _result (`/Engine/EditorBlueprintResources/StandardMacros.IncrementInt` (`self.FragmentID`))
    (:`  `
      (if (< _result (`self.TotalFragments`))
        (set `self.ActiveFragment` "BP_Fragment_")
        (bind _output_get (set `self.FragmentID` 0))
        (bind _result_2 (`/Engine/EditorBlueprintResources/StandardMacros.IncrementInt` _output_get)
          (:`  `
            (if (< _result_2 10)
              (set `self.ActiveFragment` (`KismetStringLibrary.Concat_StrStr` (`self.ActiveFragment`) "0"))
              (bind _output_get_2 (set `self.ActiveFragment` (`KismetStringLibrary.Concat_StrStr` (`self.ActiveFragment`) (`KismetStringLibrary.Conv_IntToString` (`self.FragmentID`)))))
              (`KismetSystemLibrary.PrintString` _output_get_2))))))))

(fn `UserConstructionScript`)

(fn `WorkedFragmentUpdate`
  (bind _fragmentid (`self.FragmentID`))
  (if (< _fragmentid 10)
    (set `self.ActiveFragment` (`KismetStringLibrary.Concat_StrStr` "BP_Fragment_" "0" (`KismetStringLibrary.Conv_IntToString` _fragmentid)))
    (set `self.ActiveTarget` (`KismetStringLibrary.Concat_StrStr` "BP_Target_" "0" (`KismetStringLibrary.Conv_IntToString` _fragmentid)))
    (else
      (set `self.ActiveFragment` (`KismetStringLibrary.Concat_StrStr` "BP_Fragment_" (`KismetStringLibrary.Conv_IntToString` _fragmentid)))
      (set `self.ActiveTarget` (`KismetStringLibrary.Concat_StrStr` "BP_Target_" (`KismetStringLibrary.Conv_IntToString` _fragmentid))))))