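; Clickable target slot in a mirror-repair puzzle that accepts the fragment with the same number.
; On click it compares numbers parsed from display names against BP_MirrorGame's ActiveFragment.
; A match teleports the waiting BP_Fragment onto the target, updates BP_MirrorGame's counters and active name, and slides the next fragment to the start location.
; A mismatch briefly swaps the target's material; several unconnected experimental node chains remain.
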(event `self.ReceiveActorOnClicked`
  (params (ButtonPressed :type "Key Structure"))
  (bind _fragmentid (`self.FragmentID`))
  (bind _returnvalue (`GameplayStatics.GetActorOfClass` "/Game/Blueprints/BP_MirrorGame.BP_MirrorGame_C"))
  (set `self.FragmentID` (`KismetStringLibrary.Conv_StringToInt` (`KismetStringLibrary.GetSubstring` (`/Game/Blueprints/BP_MirrorGame.ActiveFragment` _returnvalue) 12 2)))
  (set `self.TargetID` (`KismetStringLibrary.Conv_StringToInt` (`KismetStringLibrary.GetSubstring` (`KismetSystemLibrary.GetDisplayName` self) 10 2)))
  (bind _outactors (`GameplayStatics.GetAllActorsOfClass` "/Game/Blueprints/BP_Fragment.BP_Fragment_C"))
  (for _array_element _outactors
    (`KismetSystemLibrary.PrintString` "" true true (struct :`R` 0.197668 :`G` 0.765 :`A` 1.0) 10.0)
    (if (== _fragmentid (`self.TargetID`))
      (bind _returnvalue_2 (`KismetSystemLibrary.GetDisplayName` _array_element))
      (if (== (`KismetStringLibrary.Conv_StringToInt` (`KismetStringLibrary.GetSubstring` _returnvalue_2 12 2)) _fragmentid)
        (`KismetSystemLibrary.PrintString` (`KismetStringLibrary.Concat_StrStr` "this is found" _returnvalue_2) true true (struct :`G` 0.66 :`B` 1.0 :`A` 1.0) 10.0)
        (bind _returnvalue_3 (`GameplayStatics.GetActorOfClass` "/Game/Blueprints/BP_MirrorGame.BP_MirrorGame_C"))
        (if (`KismetMathLibrary.EqualExactly_VectorVector` (`self.K2_GetActorLocation` _array_element) (`/Game/Blueprints/BP_MirrorGame.FragmentStartLocation` _returnvalue_3))
          ;[1 1 1] Repairing mirror
          (`self.K2_SetActorLocation` _array_element (`self.K2_GetActorLocation` self) false false)
          (`PrimitiveComponent.SetMaterial` (`/Game/Blueprints/BP_Fragment.Fragment` _array_element) 0 "/Engine/VREditor/LaserPointer/LaserPointerMaterial_Inst.LaserPointerMaterial_Inst")
          (`KismetSystemLibrary.PrintString` "update n fragmnts" true true (struct :`G` 0.66 :`B` 1.0 :`A` 1.0) 10.0)
          (bind _fragmentsonmirror (`/Game/Blueprints/BP_MirrorGame.FragmentsOnMirror` _returnvalue_3))
          (`KismetSystemLibrary.PrintString` (`KismetStringLibrary.Conv_IntToString` _fragmentsonmirror) true true (struct :`G` 0.66 :`B` 1.0 :`A` 1.0) 10.0)
          (bind _result (`/Engine/EditorBlueprintResources/StandardMacros.IncrementInt` (`/Game/Blueprints/BP_MirrorGame.FragmentsOnMirror` _returnvalue_3))
            (:`  `
              (set `/Game/Blueprints/BP_MirrorGame.FragmentsOnMirror` _result _returnvalue_3)
              (`KismetSystemLibrary.PrintString` (`KismetStringLibrary.Conv_IntToString` _fragmentsonmirror) true true (struct :`G` 0.66 :`B` 1.0 :`A` 1.0) 10.0)
              (`GameplayStatics.PlaySound2D` "/Engine/VREditor/Sounds/VR_open.VR_open" 1.0 1.0 0.0 null null)
              (`KismetSystemLibrary.PrintString` "fragment repaired" true true (struct :`G` 0.66 :`B` 1.0 :`A` 1.0) 10.0)
              (bind _returnvalue_4 (`GameplayStatics.GetActorOfClass` "/Game/Blueprints/BP_MirrorGame.BP_MirrorGame_C"))
              (bind _result_2 (`/Engine/EditorBlueprintResources/StandardMacros.IncrementInt` (`/Game/Blueprints/BP_MirrorGame.FragmentID` _returnvalue_4))
                (:`  `
                  (bind _output_get (set `/Game/Blueprints/BP_MirrorGame.FragmentID` _result_2 _returnvalue_4))
                  (`KismetSystemLibrary.PrintString` (`KismetStringLibrary.Concat_StrStr` "fragment update" (`KismetStringLibrary.Conv_IntToString` _output_get)) true true (struct :`G` 0.66 :`B` 1.0 :`A` 1.0) 10.0)
                  (bind _fragmentid_2 (`/Game/Blueprints/BP_MirrorGame.FragmentID` _returnvalue_4))
                  (if (> _fragmentid_2 9)
                    (bind _returnvalue_5 (`KismetStringLibrary.Conv_IntToString` _fragmentid_2))
                    (set `/Game/Blueprints/BP_MirrorGame.ActiveFragment` (`KismetStringLibrary.Concat_StrStr` "BP_Fragment_" _returnvalue_5) _returnvalue_4)
                    (else
                      (set `/Game/Blueprints/BP_MirrorGame.ActiveFragment` (`KismetStringLibrary.Concat_StrStr` "BP_Fragment_" "0" _returnvalue_5) _returnvalue_4)))
                  (`KismetSystemLibrary.PrintString` (`KismetStringLibrary.Concat_StrStr` "final result is " (`/Game/Blueprints/BP_MirrorGame.ActiveFragment` _returnvalue_4)) true true (struct :`G` 0.66 :`B` 1.0 :`A` 1.0) 10.0)
                  (bind _outactors_2 (`GameplayStatics.GetAllActorsOfClass` "/Game/Blueprints/BP_Fragment.BP_Fragment_C"))
                  (for _array_element_2 _outactors_2
                    (bind _returnvalue_6 (`KismetSystemLibrary.GetDisplayName` _array_element_2))
                    (bind _activefragment (`/Game/Blueprints/BP_MirrorGame.ActiveFragment` _returnvalue_4))
                    (if (`KismetStringLibrary.EqualEqual_StrStr` _returnvalue_6 _activefragment)
                      (`KismetSystemLibrary.PrintString` (`KismetStringLibrary.Concat_StrStr` "check" _returnvalue_6 _activefragment) true true (struct :`R` 0.92443 :`G` 0.97 :`A` 1.0) 10.0)
                      (`KismetSystemLibrary.PrintString` (`KismetStringLibrary.Concat_StrStr` "ready to move" _returnvalue_6) true true (struct :`R` 1.0 :`G` 0.021249 :`B` 0.186233 :`A` 1.0) 10.0)
                      (bind _returnvalue_7 (`GameplayStatics.GetActorOfClass` "/Game/Blueprints/BP_MirrorGame.BP_MirrorGame_C"))
                      (bind _fragmentsonmirror_2 (`/Game/Blueprints/BP_MirrorGame.FragmentsOnMirror` _returnvalue_7))
                      (`KismetSystemLibrary.PrintString` (`KismetStringLibrary.Concat_StrStr` "n frammento" (`KismetStringLibrary.Conv_IntToString` _fragmentsonmirror_2)))
                      (if (< _fragmentsonmirror_2 (`/Game/Blueprints/BP_MirrorGame.TotalFragments` _returnvalue_7))
                        (`KismetSystemLibrary.MoveComponentTo` (`/Game/Blueprints/BP_Fragment.DefaultSceneRoot` _array_element_2) (`/Game/Blueprints/BP_MirrorGame.FragmentStartLocation` _returnvalue_4) (struct) false false 0.5)
                        (`KismetSystemLibrary.PrintString` (`KismetStringLibrary.Concat_StrStr` "raggiunto lo step successivo" (`KismetSystemLibrary.GetDisplayName` _array_element_2))))))))))))
      (else
        ;[1 1 1] Error
        (`PrimitiveComponent.SetMaterial` (`self.Target`) 0 "/Engine/VREditor/LaserPointer/LaserPointerMaterial.LaserPointerMaterial")
        (`KismetSystemLibrary.Delay` 3.0)
        (`PrimitiveComponent.SetMaterial` (`self.Target`) 0 "/Game/Blueprints/NormalTarget.NormalTarget")))))

(event `self.ReceiveBeginPlay`
  (`PrimitiveComponent.SetMaterial` (`self.Target`) 0 "/Game/Blueprints/NormalTarget.NormalTarget"))

(fn `UserConstructionScript`)